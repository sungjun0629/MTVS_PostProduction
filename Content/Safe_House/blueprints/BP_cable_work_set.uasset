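; Spline-driven cable set piece for the Safe House, building a cable or cable tray with fittings at both ends.
; The construction script adds a spline mesh per segment, using the small cable, big cable or tray mesh chosen by CableType.
; It places a clamp, outlet shelf or plug mesh at each end, aligned to the spline tangent with its own type and scale, flipping the end piece 180 degrees.
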(fn `UserConstructionScript`
  (locals (small_cable :type "Actor Object Reference") (big_cable :type "Actor Object Reference"))
  (bind _end_connection_scale (`self.End Connection Scale`))
  (bind _spline (`self.Spline`))
  (bind _start_connection_scale (`self.Start Connection Scale`))
  (bind (_location _tangent) (`SplineComponent.GetLocationAndTangentAtSplinePoint` (`self.Spline`) 0 "Local"))
  (bind (_location_2 _tangent_2) (`SplineComponent.GetLocationAndTangentAtSplinePoint` _spline (`SplineComponent.GetNumberOfSplinePoints` _spline) "Local"))
  (for _index (range (+ (- (`SplineComponent.GetNumberOfSplinePoints` (`self.Spline`)) 2) 1))
    (bind _returnvalue (`AddComponent|NODE_AddSplineMeshComponent-1`))
    (`StaticMeshComponent.SetStaticMesh` _returnvalue (`|GetArrayItem` (`|MakeArray` "/Game/Safe_House/meshes/SM_cable_work_cable_small.SM_cable_work_cable_small" "/Game/Safe_House/meshes/SM_cable_work_cable_big.SM_cable_work_cable_big" "/Game/Safe_House/meshes/SM_cable_work_cable_tray.SM_cable_work_cable_tray" :!type "StaticMesh Object Reference") (`KismetMathLibrary.Conv_ByteToInt` (`self.Cable Type`))))
    (`SceneComponent.K2_AttachToComponent` _returnvalue (`self.DefaultSceneRoot`) "None" "KeepRelative" "KeepRelative" "KeepRelative" true)
    (bind (_location_3 _tangent_3) (`SplineComponent.GetLocationAndTangentAtSplinePoint` (`self.Spline`) _index "Local"))
    (bind (_location_4 _tangent_4) (`SplineComponent.GetLocationAndTangentAtSplinePoint` (`self.Spline`) (+ _index 1) "Local"))
    (`SplineMeshComponent.SetStartAndEnd` _returnvalue _location_3 _tangent_3 _location_4 _tangent_4 true))
  (bind _returnvalue_2 (`AddComponent|NODE_AddStaticMeshComponent-0` :`RelativeTransform` (`KismetMathLibrary.MakeTransform` _location (`KismetMathLibrary.Conv_VectorToRotator` _tangent))))
  (`StaticMeshComponent.SetStaticMesh` _returnvalue_2 (`|GetArrayItem` (`|MakeArray` "/Game/Safe_House/meshes/SM_cable_work_clamp.SM_cable_work_clamp" "/Game/Safe_House/meshes/SM_cable_work_outlet_shelf.SM_cable_work_outlet_shelf" "/Game/Safe_House/meshes/SM_cable_work_power_plug_01.SM_cable_work_power_plug_01" "/Game/Safe_House/meshes/SM_cable_work_power_plug_02.SM_cable_work_power_plug_02" null :!type "StaticMesh Object Reference") (`KismetMathLibrary.Conv_ByteToInt` (`self.Start Connection Type`))))
  (`SceneComponent.SetRelativeScale3D` _returnvalue_2 (`KismetMathLibrary.MakeVector` _start_connection_scale _start_connection_scale _start_connection_scale))
  (bind _returnvalue_3 (`AddComponent|NODE_AddStaticMeshComponent-1` :`RelativeTransform` (`KismetMathLibrary.MakeTransform` _location_2 (`KismetMathLibrary.Conv_VectorToRotator` _tangent_2))))
  (`StaticMeshComponent.SetStaticMesh` _returnvalue_3 (`|GetArrayItem` (`|MakeArray` "/Game/Safe_House/meshes/SM_cable_work_clamp.SM_cable_work_clamp" "/Game/Safe_House/meshes/SM_cable_work_outlet_shelf.SM_cable_work_outlet_shelf" "/Game/Safe_House/meshes/SM_cable_work_power_plug_01.SM_cable_work_power_plug_01" "/Game/Safe_House/meshes/SM_cable_work_power_plug_02.SM_cable_work_power_plug_02" null :!type "StaticMesh Object Reference") (`KismetMathLibrary.Conv_ByteToInt` (`self.End Conncetion Type`))))
  (`SceneComponent.K2_AddLocalRotation` _returnvalue_3 (struct :`Yaw` 180.0) false false)
  (`SceneComponent.SetRelativeScale3D` _returnvalue_3 (`KismetMathLibrary.MakeVector` _end_connection_scale _end_connection_scale _end_connection_scale)))