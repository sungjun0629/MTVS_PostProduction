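; BP_MH_shopping is a character Blueprint that moves a mask pivot between the character's hand and head.
; Two custom events, socketToHand and socketToHead, reattach MaskPivot to the hand_l socket on Body or the horn socket on Face.
; Both keep world location, rotation and scale, so the pivot holds its current pose instead of snapping to the socket.
; Tick and the construction script only call their parents, and nothing in this Blueprint calls the two events.
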(event `self.ReceiveTick`
  (params (DeltaSeconds :type "Float (single-precision)"))
  (`parent.ReceiveTick` DeltaSeconds))

(event `socketToHand`
  (`SceneComponent.K2_AttachToComponent` (`self.Mask_Pivot`) (`self.Body`) "hand_l" "KeepWorld" "KeepWorld" "KeepWorld" true))

(event `socketToHead`
  (`SceneComponent.K2_AttachToComponent` (`self.Mask_Pivot`) (`self.Face`) "horn" "KeepWorld" "KeepWorld" "KeepWorld" true))

(fn `UserConstructionScript`
  (`parent.UserConstructionScript`))